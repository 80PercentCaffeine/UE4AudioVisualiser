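; Audio visualizer actor that rescales its components every Tick from values read on a MusicPlayerAndDecomposer reference.
; Ten cubes stretch on Z by per-channel frequency or amplitude, chosen by the FrequencyRatherThanAmplitude flag.
; Lows, Mids, Highs and Total scale uniformly with band and total intensity.
; LowsAVG, MidsAVG and HighsAVG scale by each band divided by its average, with no guard against zero.
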(event EventBeginPlay)

(event Collision|EventActorBeginOverlap
  (params (OtherActor :type Actor%20Object%20Reference)))

(event EventTick
  (params (DeltaSeconds :type Float%20%28single-precision%29))
  (bind _musicplayeranddecomposer (Variables|Default|GetMusicPlayerAndDecomposer))
  (bind _totalfrequencyintensity (Variables|/Game/MusicPlayerAndDecomposer.MusicPlayerAndDecomposer_C|GetTotalFrequencyIntensity _musicplayeranddecomposer))
  (bind _highfrequencies (Variables|/Game/MusicPlayerAndDecomposer.MusicPlayerAndDecomposer_C|GetHighFrequencies _musicplayeranddecomposer))
  (bind _lowfrequencies (Variables|/Game/MusicPlayerAndDecomposer.MusicPlayerAndDecomposer_C|GetLowFrequencies _musicplayeranddecomposer))
  (bind _midfrequencies (Variables|/Game/MusicPlayerAndDecomposer.MusicPlayerAndDecomposer_C|GetMidFrequencies _musicplayeranddecomposer))
  (bind _averagehigh (Variables|/Game/MusicPlayerAndDecomposer.MusicPlayerAndDecomposer_C|GetAverageHigh _musicplayeranddecomposer))
  (bind _averagelow (Variables|/Game/MusicPlayerAndDecomposer.MusicPlayerAndDecomposer_C|GetAverageLow _musicplayeranddecomposer))
  (bind _averagemid (Variables|/Game/MusicPlayerAndDecomposer.MusicPlayerAndDecomposer_C|GetAverageMid _musicplayeranddecomposer))
  (bind _lowfrequencies_2 (Variables|/Game/MusicPlayerAndDecomposer.MusicPlayerAndDecomposer_C|GetLowFrequencies _musicplayeranddecomposer))
  (bind _midfrequencies_2 (Variables|/Game/MusicPlayerAndDecomposer.MusicPlayerAndDecomposer_C|GetMidFrequencies _musicplayeranddecomposer))
  (bind _highfrequencies_2 (Variables|/Game/MusicPlayerAndDecomposer.MusicPlayerAndDecomposer_C|GetHighFrequencies _musicplayeranddecomposer))
  (bind _returnvalue (/ _highfrequencies_2 _averagehigh))
  (bind _returnvalue_2 (/ _lowfrequencies_2 _averagelow))
  (bind _returnvalue_3 (/ _midfrequencies_2 _averagemid))
  (if (Variables|Default|GetFrequencyRatherThanAmplitude)
    (Transformation|SetRelativeScale3D (Variables|Default|GetCube1) (Math|Vector|MakeVector 1.0 1.0 (Variables|/Game/MusicPlayerAndDecomposer.MusicPlayerAndDecomposer_C|GetCh0Frequency _musicplayeranddecomposer)))
    (Transformation|SetRelativeScale3D (Variables|Default|GetCube2) (Math|Vector|MakeVector 1.0 1.0 (Variables|/Game/MusicPlayerAndDecomposer.MusicPlayerAndDecomposer_C|GetCh1Frequency _musicplayeranddecomposer)))
    (Transformation|SetRelativeScale3D (Variables|Default|GetCube3) (Math|Vector|MakeVector 1.0 1.0 (Variables|/Game/MusicPlayerAndDecomposer.MusicPlayerAndDecomposer_C|GetCh2Frequency _musicplayeranddecomposer)))
    (Transformation|SetRelativeScale3D (Variables|Default|GetCube4) (Math|Vector|MakeVector 1.0 1.0 (Variables|/Game/MusicPlayerAndDecomposer.MusicPlayerAndDecomposer_C|GetCh3Frequency _musicplayeranddecomposer)))
    (Transformation|SetRelativeScale3D (Variables|Default|GetCube5) (Math|Vector|MakeVector 1.0 1.0 (Variables|/Game/MusicPlayerAndDecomposer.MusicPlayerAndDecomposer_C|GetCh4Frequency _musicplayeranddecomposer)))
    (Transformation|SetRelativeScale3D (Variables|Default|GetCube6) (Math|Vector|MakeVector 1.0 1.0 (Variables|/Game/MusicPlayerAndDecomposer.MusicPlayerAndDecomposer_C|GetCh5Frequency _musicplayeranddecomposer)))
    (Transformation|SetRelativeScale3D (Variables|Default|GetCube7) (Math|Vector|MakeVector 1.0 1.0 (Variables|/Game/MusicPlayerAndDecomposer.MusicPlayerAndDecomposer_C|GetCh6Frequency _musicplayeranddecomposer)))
    (Transformation|SetRelativeScale3D (Variables|Default|GetCube8) (Math|Vector|MakeVector 1.0 1.0 (Variables|/Game/MusicPlayerAndDecomposer.MusicPlayerAndDecomposer_C|GetCh7Frequency _musicplayeranddecomposer)))
    (Transformation|SetRelativeScale3D (Variables|Default|GetCube9) (Math|Vector|MakeVector 1.0 1.0 (Variables|/Game/MusicPlayerAndDecomposer.MusicPlayerAndDecomposer_C|GetCh8Frequency _musicplayeranddecomposer)))
    (Transformation|SetRelativeScale3D (Variables|Default|GetCube10) (Math|Vector|MakeVector 1.0 1.0 (Variables|/Game/MusicPlayerAndDecomposer.MusicPlayerAndDecomposer_C|GetCh9Frequency _musicplayeranddecomposer)))
    (else
      (Transformation|SetRelativeScale3D (Variables|Default|GetCube1) (Math|Vector|MakeVector 1.0 1.0 (Variables|/Game/MusicPlayerAndDecomposer.MusicPlayerAndDecomposer_C|GetCh0Amplitude _musicplayeranddecomposer)))
      (Transformation|SetRelativeScale3D (Variables|Default|GetCube2) (Math|Vector|MakeVector 1.0 1.0 (Variables|/Game/MusicPlayerAndDecomposer.MusicPlayerAndDecomposer_C|GetCh1Amplitude _musicplayeranddecomposer)))
      (Transformation|SetRelativeScale3D (Variables|Default|GetCube3) (Math|Vector|MakeVector 1.0 1.0 (Variables|/Game/MusicPlayerAndDecomposer.MusicPlayerAndDecomposer_C|GetCh2Amplitude _musicplayeranddecomposer)))
      (Transformation|SetRelativeScale3D (Variables|Default|GetCube4) (Math|Vector|MakeVector 1.0 1.0 (Variables|/Game/MusicPlayerAndDecomposer.MusicPlayerAndDecomposer_C|GetCh3Amplitude _musicplayeranddecomposer)))
      (Transformation|SetRelativeScale3D (Variables|Default|GetCube5) (Math|Vector|MakeVector 1.0 1.0 (Variables|/Game/MusicPlayerAndDecomposer.MusicPlayerAndDecomposer_C|GetCh4Amplitude _musicplayeranddecomposer)))
      (Transformation|SetRelativeScale3D (Variables|Default|GetCube6) (Math|Vector|MakeVector 1.0 1.0 (Variables|/Game/MusicPlayerAndDecomposer.MusicPlayerAndDecomposer_C|GetCh5Amplitude _musicplayeranddecomposer)))
      (Transformation|SetRelativeScale3D (Variables|Default|GetCube7) (Math|Vector|MakeVector 1.0 1.0 (Variables|/Game/MusicPlayerAndDecomposer.MusicPlayerAndDecomposer_C|GetCh6Amplitude _musicplayeranddecomposer)))
      (Transformation|SetRelativeScale3D (Variables|Default|GetCube8) (Math|Vector|MakeVector 1.0 1.0 (Variables|/Game/MusicPlayerAndDecomposer.MusicPlayerAndDecomposer_C|GetCh7Amplitude _musicplayeranddecomposer)))
      (Transformation|SetRelativeScale3D (Variables|Default|GetCube9) (Math|Vector|MakeVector 1.0 1.0 (Variables|/Game/MusicPlayerAndDecomposer.MusicPlayerAndDecomposer_C|GetCh8Amplitude _musicplayeranddecomposer)))
      (Transformation|SetRelativeScale3D (Variables|Default|GetCube10) (Math|Vector|MakeVector 1.0 1.0 (Variables|/Game/MusicPlayerAndDecomposer.MusicPlayerAndDecomposer_C|GetCh9Amplitude _musicplayeranddecomposer)))))
  (Transformation|SetRelativeScale3D (Variables|Default|GetLows) (Math|Vector|MakeVector _lowfrequencies _lowfrequencies _lowfrequencies))
  (Transformation|SetRelativeScale3D (Variables|Default|GetHighs) (Math|Vector|MakeVector _highfrequencies _highfrequencies _highfrequencies))
  (Transformation|SetRelativeScale3D (Variables|Default|GetMids) (Math|Vector|MakeVector _midfrequencies _midfrequencies _midfrequencies))
  (Transformation|SetRelativeScale3D (Variables|Default|GetTotal) (Math|Vector|MakeVector _totalfrequencyintensity _totalfrequencyintensity _totalfrequencyintensity))
  (Transformation|SetRelativeScale3D (Variables|Default|GetLowsAVG) (Math|Vector|MakeVector _returnvalue_2 _returnvalue_2 _returnvalue_2))
  (Transformation|SetRelativeScale3D (Variables|Default|GetMidsAVG) (Math|Vector|MakeVector _returnvalue_3 _returnvalue_3 _returnvalue_3))
  (Transformation|SetRelativeScale3D (Variables|Default|GetHighsAVG) (Math|Vector|MakeVector _returnvalue _returnvalue _returnvalue)))

(fn ConstructionScript)